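; BP_Weapon is a firearm that spawns BP_Bullet actors from its skeletal mesh's Muzzle socket, with a particle effect and AK47 shot sound.
; StartFire branches on FireMod: Single fires once, while Auto plays the AutoFire timeline, whose Fire event track triggers each shot.
; StopFire resets and stops that timeline, and FireModeSwitch toggles between the two modes.
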(event `Start Fire`
  (bind _muzzlerotation (`self.MuzzleRotation`))
  (bind _location (.location (`SceneComponent.GetSocketTransform` (`self.SkeletalMesh`) "Muzzle" "RTS_World")))
  (switch `/Game/Blueprints/Fire_Modes` (`self.FireMod`)
    (:`NewEnumerator0`
      (`AddComponent|NODE_AddParticleSystemComponent-0` :`bManualAttachment` true :`RelativeTransform` (`KismetMathLibrary.MakeTransform` _location _muzzlerotation (0.2 0.2 0.2)))
      (`GameplayStatics.PlaySoundAtLocation` "/Game/Sounds/AK47_ShootSFX.AK47_ShootSFX" _location (struct) 1.0 1.0 0.0 null null null)
      (`|SpawnActorFromClass` "/Game/Blueprints/BP_Bullet.BP_Bullet_C" (`KismetMathLibrary.MakeTransform` _location _muzzlerotation (1.0 1.0 1.0)) "AlwaysSpawn" "OverrideRootScale" null null :!label _label))
    (:`NewEnumerator1`
      (`Timeline|AutoFire` :!label _label_2
        (:`Fire`
          (`AddComponent|NODE_AddParticleSystemComponent-2` :`bManualAttachment` true :`RelativeTransform` (`KismetMathLibrary.MakeTransform` _location _muzzlerotation (0.2 0.2 0.2)))
          (`GameplayStatics.PlaySoundAtLocation` "/Game/Sounds/AK47_ShootSFX.AK47_ShootSFX" _location (struct) 1.0 1.0 0.0 null null null)
          (goto _label))))))

(event `Stop Fire`
  (`|ExecutionSequence`
    (:`then_0`
      (goto _label_2 :!via `SetNewTime`))
    (:`then_1`
      (goto _label_2 :!via `Stop`))))

(fn `FireModeSwitch`
  (switch `/Game/Blueprints/Fire_Modes` (`self.FireMod`)
    (:`NewEnumerator0`
      (set `self.FireMod` "NewEnumerator1"))
    (:`NewEnumerator1`
      (set `self.FireMod` "NewEnumerator0"))))

(fn `UserConstructionScript`
  (`parent.UserConstructionScript`))